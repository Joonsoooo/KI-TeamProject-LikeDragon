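; Ryoma character Blueprint that manages his HUD widgets and battle presentation.
; BeginPlay creates subtitle, status, minimap and win/lose widgets, then binds to DefaultGameState combat changes and the UI component's Hact gauge.
; A full gauge during combat lights two Niagara auras, while victory triggers sound, post-process material, timeline-driven time dilation and win screen.
; Functions toggle widgets and load DataTable cutscene text; number keys force battle start and result screens.
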(event `self.ReceiveBeginPlay`
  (bind _returnvalue (`GameplayStatics.GetPlayerController` 0))
  (`|ExecutionSequence`
    (:`then_0`
      (bind _returnvalue_2 (`|CreateWidget` "/Game/Like/BP_/WIdget/WBP_SequenceTextBox.WBP_SequenceTextBox_C" _returnvalue))
      (bind _output_get (set `self.WBP_SqWidget` _returnvalue_2))
      (`UserWidget.AddToViewport` _output_get 0)
      (`Widget.SetVisibility` (`self.WBP_SqWidget`) "Hidden"))
    (:`then_1`
      (bind _returnvalue_3 (`|CreateWidget` "/Game/Like/BP_/WIdget/Ryoma/WBP_RyomaStatus.WBP_RyomaStatus_C" _returnvalue))
      (set `self.WBP_RyomaStatus` _returnvalue_3))
    (:`then_2`
      (bind _returnvalue_4 (`|CreateWidget` "/Game/Like/BP_/WIdget/Battle/WBP_BattleWin.WBP_BattleWin_C" _returnvalue))
      (set `self.WBP_BattleWIn` _returnvalue_4))
    (:`then_3`
      (bind _returnvalue_5 (`|CreateWidget` "/Game/Like/BP_/WIdget/Battle/WBP_BattleLose.WBP_BattleLose_C" _returnvalue))
      (set `self.WBP_BattleLose` _returnvalue_5))
    (:`then_4`
      (bind _returnvalue_6 (`|CreateWidget` "/Game/Like/BP_/WIdget/WBP_Minimap.WBP_Minimap_C" _returnvalue))
      (bind _output_get_2 (set `self.WBP_Minimap` _returnvalue_6))
      (`UserWidget.AddToViewport` _output_get_2 0)
      (bind _asdefault_game_state (cast `DefaultGameState` (`GameplayStatics.GetGameState`)))
      (set `self.As Default Game State` _asdefault_game_state)
      (add `DefaultGameState.SetCombatGameStateChanged` _asdefault_game_state (delegate `SetCombatGameStateChanged_Event`))
      (bind _returnvalue_7 (`KismetMaterialLibrary.CreateDynamicMaterialInstance` "/Game/Like/BP_/Materials/MI_PostProcessing_Inst.MI_PostProcessing_Inst"))
      (set `self.BattleMaterial` _returnvalue_7)
      (add `RyomaUIComponent.OnHactCurrentChanged` (`self.RyomaUIComponent`) (delegate `OnHactCurrentChanged_Event`)))))

(event `OnHactCurrentChanged_Event`
  (params (NewPercent :type "Float (single-precision)"))
  (bind _ns_aura_2 (`self.NS_Aura_2`))
  (bind _ns_aura_1 (`self.NS_Aura_1`))
  (set `self.HactCound` NewPercent)
  (bind _returnvalue (`DefaultGameState.GetCombatGameState` (`self.As Default Game State`)))
  (if (== _returnvalue 5)
    (if (`KismetMathLibrary.NearlyEqual_FloatFloat` (`self.HactCound`) 1.0)
      (`ActorComponent.Activate` _ns_aura_1 false)
      (`ActorComponent.Activate` _ns_aura_2 false)
      (else
        (`ActorComponent.Deactivate` _ns_aura_1)
        (`ActorComponent.Deactivate` _ns_aura_2)))))

(event `Key|One`
  (params (Key :type "Key Structure"))
  (:`Pressed`
    (`DefaultGameState.SetCombatGameState` (`self.As Default Game State`) "BattleStart")
    (`UserWidget.AddToViewport` (`self.WBP_RyomaStatus`) 0)
    (`self.AllEnemyDection`)))

(event `SetCombatGameStateChanged_Event`
  (params (OutCombatGameState :type "ECombatGameState Enum" :default "None"))
  (bind _ns_aura_2 (`self.NS_Aura_2`))
  (bind _ns_aura_1 (`self.NS_Aura_1`))
  (switch `int` (`KismetMathLibrary.Conv_ByteToInt` OutCombatGameState)
    (:`5`
      (if (== OutCombatGameState 5)
        (`UserWidget.AddToViewport` (`self.WBP_RyomaStatus`) 0)
        (if (`KismetMathLibrary.NearlyEqual_FloatFloat` (`self.HactCound`) 1.0)
          (`ActorComponent.Activate` _ns_aura_1 false)
          (`ActorComponent.Activate` _ns_aura_2 false)
          (else
            (`ActorComponent.Deactivate` _ns_aura_1)
            (`ActorComponent.Deactivate` _ns_aura_2)))))
    (:`6`
      (`|ExecutionSequence`
        (:`then_0`
          (`GameplayStatics.PlaySoundAtLocation` "/Game/Asset/Sound/전투/전투_종료/승리/43_kyukyoku_win__36_.43_kyukyoku_win__36_" (`self.K2_GetActorLocation`) (struct) 1.0 1.0 0.0 null null null null)
          (`MaterialInstanceDynamic.SetVectorParameterValue` (`self.BattleMaterial`) "BattleColor" (struct :`A` 1.0))
          (setmembers `PostProcessSettings` :`StructRef` (`CameraComponent.PostProcessSettings` (`self.FollowCamera`)) :`WeightedBlendables` (make `WeightedBlendables` (`|MakeArray` (make `WeightedBlendable` 1.0 (`self.BattleMaterial`)))))
          (`CameraComponent.SetPostProcessBlendWeight` (`self.FollowCamera`) 1.0))
        (:`then_1`
          (bind (_direction _newtrack_0) (`Timeline|Timeline` :!via `PlayFromStart`)
            (:`Update`
              (`GameplayStatics.SetGlobalTimeDilation` _newtrack_0)
              (`KismetSystemLibrary.Delay` 0.95)
              (`UserWidget.AddToViewport` (`self.WBP_BattleWIn`) 0))))))))

(event `self.ReceiveTick`
  (params (DeltaSeconds :type "Float (single-precision)")))

(event `Key|Six`
  (params (Key :type "Key Structure"))
  (:`Pressed`
    (`UserWidget.AddToViewport` (`self.WBP_BattleWIn`) 0)))

(event `Key|Seven`
  (params (Key :type "Key Structure"))
  (:`Pressed`
    (`UserWidget.AddToViewport` (`self.WBP_BattleLose`) 0)))

(event `Key|Five`
  (params (Key :type "Key Structure")))

(event `/Game/Like/BP_/WIdget/Interface/BPI_RyomaStatusVisible.RyomaStatusVisibleSet`
  (bind _wbp_ryomastatus (`self.WBP_RyomaStatus`))
  (`UserWidget.AddToViewport` _wbp_ryomastatus 4)
  (`/Engine/EditorBlueprintResources/StandardMacros.FlipFlop`
    (:`A`
      (`Widget.SetVisibility` _wbp_ryomastatus "HitTestInvisible"))
    (:`B`
      (`Widget.SetVisibility` _wbp_ryomastatus "Hidden")
      (`Widget.RemoveFromParent` _wbp_ryomastatus))))

(fn `Get WBP_BattleLose`
  (returns (`WBP Battle Lose` :type "/Game/Like/BP_/WIdget/Battle/WBP_BattleLose Object Reference"))
  (return (`self.WBP_BattleLose`)))

(fn `OkitaMidRyomaHpoff`
  (`Widget.SetVisibility` (`self.WBP_RyomaStatus`) "Hidden"))

(fn `OkitaMidRyomaHpOn`
  (`Widget.SetVisibility` (`self.WBP_RyomaStatus`) "Visible"))

(fn `SqMinimapOff`
  (`Widget.SetVisibility` (`self.WBP_Minimap`) "Hidden"))

(fn `SqMinimapOn`
  (`Widget.SetVisibility` (`self.WBP_Minimap`) "Visible"))

(fn `SqTextWidgetOff`
  (`Widget.SetVisibility` (`self.WBP_SqWidget`) "Hidden"))

(fn `SqTextWidgetOn`
  (bind (_st_sq_text_row_name _st_sq_text_row_text) (break `/Game/Like/BP_/DataTable/Sequence/St_SqTextRow` (`self.St Sq Text Row`)))
  ;[0 1 0.7481] Sequence Text Widget
  (bind _returnvalue (`|GetDataTableRow` "/Game/Like/BP_/DataTable/Sequence/CutSinText.CutSinText" (`KismetStringLibrary.Conv_StringToName` (`KismetStringLibrary.Conv_IntToString` (`self.Sq_RowNameIndex`))))
    (:`then`
      (set `self.St Sq Text Row` _returnvalue)
      (`Widget.SetVisibility` (`self.WBP_SqWidget`) "Visible")
      (set `/Game/Like/BP_/WIdget/WBP_SequenceTextBox.SqTextName` _st_sq_text_row_name (`self.WBP_SqWidget`))
      (set `/Game/Like/BP_/WIdget/WBP_SequenceTextBox.SqMainText` _st_sq_text_row_text (`self.WBP_SqWidget`)))
    (:`RowNotFound`
      (`KismetSystemLibrary.PrintString` "EmptyData"))))

(fn `UserConstructionScript`)