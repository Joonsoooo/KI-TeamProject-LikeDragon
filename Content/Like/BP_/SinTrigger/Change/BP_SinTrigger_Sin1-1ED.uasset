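; BP_SinTrigger_Sin1-1ED is a level-transition trigger that opens the Sin2 level when its TriggerBox is overlapped.
; A sequence first casts the overlapping actor to BP_RyomaCharacter, storing it as PlayerActor if unset and printing debug strings.
; It then destroys CreateSq and itself before opening the level.
; This second branch is not gated by the cast, so any overlapping actor triggers the transition.
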(event `self.TriggerBox.OnComponentBeginOverlap`
  (params (OverlappedComponent :type "PrimitiveComponent Object Reference") (OtherActor :type "Actor Object Reference") (OtherComp :type "PrimitiveComponent Object Reference") (OtherBodyIndex :type Integer) (bFromSweep :type Boolean) (SweepResult :type "HitResult Structure (by ref)"))
  (`|ExecutionSequence`
    (:`then_0`
      (cast `/Game/Like/BP_/Characters/Ryoma/BP_RyomaCharacter` OtherActor)
      (`/Engine/EditorBlueprintResources/StandardMacros.IsValid` (`self.PlayerActor`)
        (:`Is Valid`
          _)
        (:`Is Not Valid`
          (set `self.PlayerActor` OtherActor)))
      (`KismetSystemLibrary.PrintString` "SucceseSetPlayer")
      (`KismetSystemLibrary.PrintString` (`KismetSystemLibrary.GetDisplayName` (`self.PlayerActor`))))
    (:`then_1`
      (`self.K2_DestroyActor` (`self.CreateSq`))
      (`self.K2_DestroyActor`)
      (`GameplayStatics.OpenLevelBySoftObjectPtr` "/Game/Like/Level/Sin2/Sin2.Sin2"))))

(fn `UserConstructionScript`)