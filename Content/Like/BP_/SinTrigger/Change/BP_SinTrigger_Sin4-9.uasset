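; BP_SinTrigger_Sin4-9 reacts to combat game state changes for stage Sin 4-9, handling the minimap and level transitions.
; On BeginPlay it caches the Ryoma player character and DefaultGameState, printing debug messages, then binds two handlers to the state-change dispatcher.
; EndFight turns off the player's minimap in one state.
; EndManu opens either the Sin49 or Sin48 level, depending on the state received.
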(event `self.ReceiveBeginPlay`
  (`|ExecutionSequence`
    (:`then_0`
      (bind _asbp_ryoma_character (cast `/Game/Like/BP_/Characters/Ryoma/BP_RyomaCharacter` (`GameplayStatics.GetPlayerCharacter` 0)))
      (`/Engine/EditorBlueprintResources/StandardMacros.IsValid` (`self.PlayerActor`)
        (:`Is Valid`
          _)
        (:`Is Not Valid`
          (set `self.PlayerActor` _asbp_ryoma_character)))
      (`KismetSystemLibrary.PrintString` "SucceseSetPlayer" true true (struct :`G` 0.181602 :`B` 1.0 :`A` 1.0))
      (`KismetSystemLibrary.PrintString` (`KismetSystemLibrary.GetDisplayName` (`self.PlayerActor`))))
    (:`then_1`
      (bind _asdefault_game_state (cast `DefaultGameState` (`GameplayStatics.GetGameState`)))
      (`/Engine/EditorBlueprintResources/StandardMacros.IsValid` (`self.As Default Game State`)
        (:`Is Valid`
          _)
        (:`Is Not Valid`
          (set `self.As Default Game State` _asdefault_game_state)))
      (`KismetSystemLibrary.PrintString` "SucceseSetGameState" true true (struct :`G` 0.052697 :`B` 1.0 :`A` 1.0))
      (`KismetSystemLibrary.PrintString` (`KismetSystemLibrary.GetDisplayName` (`self.As Default Game State`))))
    (:`then_2`
      (add `DefaultGameState.SetCombatGameStateChanged` (`self.As Default Game State`) (delegate `EndFight`))
      (add `DefaultGameState.SetCombatGameStateChanged` (`self.As Default Game State`) (delegate `EndManu`)))))

(event `EndFight`
  (params (OutCombatGameState :type "ECombatGameState Enum" :default "None"))
  (if (== OutCombatGameState 6)
    (`/Game/Like/BP_/Characters/Ryoma/BP_RyomaCharacter.SqMinimapOff` (`self.PlayerActor`))))

(event `EndManu`
  (params (OutCombatGameState :type "ECombatGameState Enum" :default "None"))
  (if (== OutCombatGameState 7)
    (`GameplayStatics.OpenLevelBySoftObjectPtr` "/Game/Like/Level/Sin4/Sin4-9.Sin4-9")
    (elif (== OutCombatGameState 8)
      (`GameplayStatics.OpenLevelBySoftObjectPtr` "/Game/Like/Level/Sin4/Sin4-8.Sin4-8"))))

(fn `UserConstructionScript`)