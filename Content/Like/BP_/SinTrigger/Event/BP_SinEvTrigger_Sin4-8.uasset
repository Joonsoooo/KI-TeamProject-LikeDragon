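; Event trigger actor that plays the Sin48 level sequence as a cutscene on BeginPlay and then starts a battle.
; After a short delay it caches the player and EnemyPivot, turns off the minimap, then hides and moves the player to a hidden point.
; When the sequence finishes, it repositions player, camera and EnemyPivot, sets combat state to BattleStart, restores the minimap, calls battle sound, and destroys itself.
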(event `self.ReceiveBeginPlay`
  (`KismetSystemLibrary.Delay` 0.2)
  (`|ExecutionSequence`
    (:`then_0`
      (bind _asbp_ryoma_character (cast `/Game/Like/BP_/Characters/Ryoma/BP_RyomaCharacter` (`GameplayStatics.GetPlayerCharacter` 0)))
      (`/Engine/EditorBlueprintResources/StandardMacros.IsValid` (`self.PlayerActor`)
        (:`Is Valid`
          _)
        (:`Is Not Valid`
          (set `self.PlayerActor` _asbp_ryoma_character)))
      (`KismetSystemLibrary.PrintString` "SucceseSetPlayer")
      (`KismetSystemLibrary.PrintString` (`KismetSystemLibrary.GetDisplayName` (`self.PlayerActor`)))
      (bind _returnvalue (`GameplayStatics.GetActorOfClass` "/Game/Like/BP_/Enemy/MeleeEnemy/EnemyPivot.EnemyPivot_C"))
      (set `self.EnemyPivot` _returnvalue))
    (:`then_1`
      (`/Game/Like/BP_/Characters/Ryoma/BP_RyomaCharacter.SqMinimapOff` (`self.PlayerActor`))
      (`self.SetActorHiddenInGame` (`self.PlayerActor`) true)
      (`self.K2_SetActorTransform` (`self.PlayerActor`) (`self.HiddenPoint`) false true))
    (:`then_2`
      (bind _outactor (`LevelSequencePlayer.CreateLevelSequencePlayer` "/Game/Like/Sequence/Sin4-8.Sin4-8"))
      (set `self.CreateSq` _outactor)
      (`MovieSceneSequencePlayer.Play` (`LevelSequenceActor.SequencePlayer` (`self.CreateSq`))))
    (:`then_3`
      (add `MovieSceneSequencePlayer.OnFinished` (`LevelSequenceActor.SequencePlayer` (`self.CreateSq`)) (delegate `OnFinished_Event`)))))

(event `OnFinished_Event`
  (bind _returnvalue (`self.GetTransform` (`self.EnemyPivot`)))
  (`self.K2_SetActorTransform` (`self.PlayerActor`) (`self.End Point`) false true)
  (`self.K2_SetActorTransform` (`GameplayStatics.GetPlayerCameraManager` 0) (`self.PlayerCameraPoint`) false false)
  (`self.SetActorHiddenInGame` (`self.PlayerActor`) false)
  (`self.K2_SetActorTransform` (`self.EnemyPivot`) (`KismetMathLibrary.MakeTransform` (`KismetMathLibrary.MakeVector` (.x (.location _returnvalue)) (.y (.location _returnvalue)) 200.0) (.rotation _returnvalue) (.scale _returnvalue)) false true)
  (`|ExecutionSequence`
    (:`then_0`
      (bind _asdefault_game_state (cast `DefaultGameState` (`GameplayStatics.GetGameState`)))
      (`DefaultGameState.SetCombatGameState` _asdefault_game_state "BattleStart")
      (`/Game/Like/BP_/Characters/Ryoma/BP_RyomaCharacter.SqMinimapOn` (`self.PlayerActor`))
      (`self.BattleSound4`))
    (:`then_1`
      (`self.K2_DestroyActor` (`self.CreateSq`))
      (`self.K2_DestroyActor`))))

(fn `UserConstructionScript`)