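; Scene event actor for Sin2-1 that plays three level sequences back to back after a short BeginPlay delay.
; It first turns off the player's minimap, hides the Ryoma character and teleports it to HiddenPoint.
; Each sequence's OnFinished starts the next; the last restores player, camera and minimap at end points, then destroys its sequence actor and itself.
; Puase and Play events pause and resume the current sequence.
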(event `self.ReceiveBeginPlay`
  (`KismetSystemLibrary.Delay` 0.2)
  (`|ExecutionSequence`
    (:`then_0`
      (bind _asbp_ryoma_character (cast `/Game/Like/BP_/Characters/Ryoma/BP_RyomaCharacter` (`GameplayStatics.GetPlayerCharacter` 0)))
      (`/Engine/EditorBlueprintResources/StandardMacros.IsValid` (`self.PlayerActor`)
        (:`Is Valid`
          _)
        (:`Is Not Valid`
          (set `self.PlayerActor` _asbp_ryoma_character)))
      (`KismetSystemLibrary.PrintString` "SucceseSetPlayer")
      (`KismetSystemLibrary.PrintString` (`KismetSystemLibrary.GetDisplayName` (`self.PlayerActor`)))
      (`/Game/Like/BP_/Characters/Ryoma/BP_RyomaCharacter.SqMinimapOff` (`self.PlayerActor`)))
    (:`then_1`
      (`/Game/Like/BP_/Characters/Ryoma/BP_RyomaCharacter.SqMinimapOff` (`self.PlayerActor`))
      (`self.SetActorHiddenInGame` (`self.PlayerActor`) true)
      (`self.K2_SetActorTransform` (`self.PlayerActor`) (`self.HiddenPoint`) false true))
    (:`then_2`
      (bind _outactor (`LevelSequencePlayer.CreateLevelSequencePlayer` "/Game/Like/Sequence/Sin2-1.Sin2-1"))
      (set `self.CreateSq` _outactor)
      (`MovieSceneSequencePlayer.Play` (`LevelSequenceActor.SequencePlayer` (`self.CreateSq`)))
      (add `MovieSceneSequencePlayer.OnFinished` (`LevelSequenceActor.SequencePlayer` (`self.CreateSq`)) (delegate `Q1End`)))))

(event `Q1End`
  (`self.Q2`))

(event `Q2`
  (bind _outactor (`LevelSequencePlayer.CreateLevelSequencePlayer` "/Game/Like/Sequence/Sin2-2.Sin2-2"))
  (set `self.CreateSq` _outactor)
  (`MovieSceneSequencePlayer.Play` (`LevelSequenceActor.SequencePlayer` (`self.CreateSq`)))
  (add `MovieSceneSequencePlayer.OnFinished` (`LevelSequenceActor.SequencePlayer` (`self.CreateSq`)) (delegate `Q2End`)))

(event `Q2End`
  (`self.Q3`))

(event `Q3`
  (bind _outactor (`LevelSequencePlayer.CreateLevelSequencePlayer` "/Game/Like/Sequence/Sin2-3.Sin2-3"))
  (set `self.CreateSq` _outactor)
  (`MovieSceneSequencePlayer.Play` (`LevelSequenceActor.SequencePlayer` (`self.CreateSq`)))
  (add `MovieSceneSequencePlayer.OnFinished` (`LevelSequenceActor.SequencePlayer` (`self.CreateSq`)) (delegate `Q3End`)))

(event `Q3End`
  (`self.QEnd`))

(event `QEnd`
  (`self.K2_SetActorTransform` (`self.PlayerActor`) (`self.End Point`) false true)
  (`self.K2_SetActorTransform` (`GameplayStatics.GetPlayerCameraManager` 0) (`self.PlayerCameraPoint`) false false)
  (`self.SetActorHiddenInGame` (`self.PlayerActor`) false)
  (`/Game/Like/BP_/Characters/Ryoma/BP_RyomaCharacter.SqMinimapOn` (`self.PlayerActor`))
  (`self.K2_DestroyActor` (`self.CreateSq`))
  (`self.K2_DestroyActor`))

(event `Puase`
  (`MovieSceneSequencePlayer.Pause` (`LevelSequenceActor.SequencePlayer` (`self.CreateSq`))))

(event `Play`
  (`MovieSceneSequencePlayer.Play` (`LevelSequenceActor.SequencePlayer` (`self.CreateSq`))))

(fn `UserConstructionScript`)