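; BP_SinEvTrigger_Sin4-10 is a one-shot event actor that plays the Sin410 Level Sequence shortly after BeginPlay.
; After a brief delay it caches the Ryoma player, turns off the minimap, hides the player and teleports them to a hidden point.
; When the sequence finishes, it moves the player and camera manager to preset transforms, restores visibility and minimap, then destroys the sequence actor and itself.
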(event `self.ReceiveBeginPlay`
  (`KismetSystemLibrary.Delay` 0.2)
  (`|ExecutionSequence`
    (:`then_0`
      (bind _asbp_ryoma_character (cast `/Game/Like/BP_/Characters/Ryoma/BP_RyomaCharacter` (`GameplayStatics.GetPlayerCharacter` 0)))
      (`/Engine/EditorBlueprintResources/StandardMacros.IsValid` (`self.PlayerActor`)
        (:`Is Valid`
          _)
        (:`Is Not Valid`
          (set `self.PlayerActor` _asbp_ryoma_character)))
      (`KismetSystemLibrary.PrintString` "SucceseSetPlayer")
      (`KismetSystemLibrary.PrintString` (`KismetSystemLibrary.GetDisplayName` (`self.PlayerActor`))))
    (:`then_1`
      (`/Game/Like/BP_/Characters/Ryoma/BP_RyomaCharacter.SqMinimapOff` (`self.PlayerActor`))
      (`self.SetActorHiddenInGame` (`self.PlayerActor`) true)
      (`self.K2_SetActorTransform` (`self.PlayerActor`) (`self.HiddenPoint`) false true))
    (:`then_2`
      (bind _outactor (`LevelSequencePlayer.CreateLevelSequencePlayer` "/Game/Like/Sequence/Sin4-10.Sin4-10"))
      (set `self.CreateSq` _outactor)
      (`MovieSceneSequencePlayer.Play` (`LevelSequenceActor.SequencePlayer` (`self.CreateSq`))))
    (:`then_3`
      (add `MovieSceneSequencePlayer.OnFinished` (`LevelSequenceActor.SequencePlayer` (`self.CreateSq`)) (delegate `OnFinished_Event`)))))

(event `OnFinished_Event`
  (`self.K2_SetActorTransform` (`self.PlayerActor`) (`self.End Point`) false true)
  (`self.K2_SetActorTransform` (`GameplayStatics.GetPlayerCameraManager` 0) (`self.Player Camera Point`) false false)
  (`self.SetActorHiddenInGame` (`self.PlayerActor`) false)
  (`/Game/Like/BP_/Characters/Ryoma/BP_RyomaCharacter.SqMinimapOn` (`self.PlayerActor`))
  (`self.K2_DestroyActor` (`self.CreateSq`))
  (`self.K2_DestroyActor`))

(fn `UserConstructionScript`)