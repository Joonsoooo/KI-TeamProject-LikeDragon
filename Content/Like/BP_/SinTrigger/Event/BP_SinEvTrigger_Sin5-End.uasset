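; Scene 5 event actor that starts the boss battle and plays a mid-fight cutscene when the boss reports low health.
; Shortly after BeginPlay it caches the Ryoma player, sets BattleStart, starts battle sound and binds the boss's health dispatcher.
; That event hides HUD and player, moves both fighters away and plays the Sin53 sequence.
; On finish it repositions both, restores combat and HUD, then destroys itself.
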(event `self.ReceiveBeginPlay`
  (`KismetSystemLibrary.Delay` 0.4)
  (`|ExecutionSequence`
    (:`then_0`
      (bind _asbp_ryoma_character (cast `/Game/Like/BP_/Characters/Ryoma/BP_RyomaCharacter` (`GameplayStatics.GetPlayerCharacter` 0)))
      (`/Engine/EditorBlueprintResources/StandardMacros.IsValid` (`self.PlayerActor`)
        (:`Is Valid`
          _)
        (:`Is Not Valid`
          (set `self.PlayerActor` _asbp_ryoma_character)))
      (`KismetSystemLibrary.PrintString` "SucceseSetPlayer")
      (`KismetSystemLibrary.PrintString` (`KismetSystemLibrary.GetDisplayName` (`self.PlayerActor`))))
    (:`then_1`
      (bind _asdefault_game_state (cast `DefaultGameState` (`GameplayStatics.GetGameState`)))
      (`DefaultGameState.SetCombatGameState` _asdefault_game_state "BattleStart")
      (`/Game/Like/BP_/Characters/Ryoma/BP_RyomaCharacter.SqMinimapOn` (`self.PlayerActor`))
      (`self.BattleSound5`))
    (:`then_2`
      (bind _returnvalue (`GameplayStatics.GetActorOfClass` "/Game/Like/BP_/Enemy/Boss/BP_Boss.BP_Boss_C"))
      (bind _output_get (set `self.Boss` _returnvalue))
      (add `EnemyCharacter.GetCurrentedBossHealth` _output_get (delegate `GetCurrentedBossHealth_Event`)))))

(event `GetCurrentedBossHealth_Event`
  (bind _boss (`self.Boss`))
  (bind _returnvalue (`self.GetTransform` _boss))
  (`KismetSystemLibrary.PrintString` "Low Hp")
  (`|ExecutionSequence`
    (:`then_1`
      (`/Game/Like/BP_/Characters/Ryoma/BP_RyomaCharacter.OkitaMidRyomaHpoff` (`self.PlayerActor`))
      (`/Game/Like/BP_/Characters/Ryoma/BP_RyomaCharacter.SqMinimapOff` (`self.PlayerActor`))
      (`self.SetActorHiddenInGame` (`self.PlayerActor`) true)
      (`self.K2_SetActorTransform` (`self.PlayerActor`) (`self.HiddenPoint`) false true)
      (`self.K2_SetActorTransform` _boss (`KismetMathLibrary.MakeTransform` (`KismetMathLibrary.MakeVector` (.x (.location _returnvalue)) (.y (.location _returnvalue)) -4000.0) (.rotation _returnvalue) (.scale _returnvalue)) false true))
    (:`then_2`
      (bind _outactor (`LevelSequencePlayer.CreateLevelSequencePlayer` "/Game/Like/Sequence/Sin5-3.Sin5-3"))
      (set `self.CreateSq` _outactor)
      (`MovieSceneSequencePlayer.Play` (`LevelSequenceActor.SequencePlayer` (`self.CreateSq`))))
    (:`then_3`
      (add `MovieSceneSequencePlayer.OnFinished` (`LevelSequenceActor.SequencePlayer` (`self.CreateSq`)) (delegate `OnFinished_Event`)))))

(event `OnFinished_Event`
  (bind _boss (`self.Boss`))
  (`self.K2_SetActorTransform` (`self.PlayerActor`) (`self.End Point`) false true)
  (`self.K2_SetActorTransform` (`GameplayStatics.GetPlayerCameraManager` 0) (`self.PlayerCameraPoint`) false false)
  (`self.SetActorHiddenInGame` (`self.PlayerActor`) false)
  (`self.K2_SetActorTransform` _boss (`KismetMathLibrary.MakeTransform` (6401.0 2569.0 517.0) (struct) (.scale (`self.GetTransform` _boss))) false true)
  (`self.SetActorHiddenInGame` _boss false)
  (`|ExecutionSequence`
    (:`then_0`
      (bind _asdefault_game_state (cast `DefaultGameState` (`GameplayStatics.GetGameState`)))
      (`DefaultGameState.SetCombatGameState` _asdefault_game_state "BattleStart")
      (`/Game/Like/BP_/Characters/Ryoma/BP_RyomaCharacter.SqMinimapOn` (`self.PlayerActor`))
      (`/Game/Like/BP_/Characters/Ryoma/BP_RyomaCharacter.OkitaMidRyomaHpOn` (`self.PlayerActor`)))
    (:`then_1`
      (`self.K2_DestroyActor` (`self.CreateSq`))
      (`self.K2_DestroyActor`))))

(fn `UserConstructionScript`)