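; BP_RangedBadguys is a ranged enemy Blueprint for a thug ("불량배") built on a parent enemy class.
; On BeginPlay it runs the parent logic, then writes that name into the enemy health bar widget.
; A Hit event, commented as a sword-hit test, briefly swaps one kimono material slot to a test material and restores it after a short delay.
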(event `self.ReceiveBeginPlay`
  (`parent.ReceiveBeginPlay`)
  (`TextBlock.SetText` (`/Game/Like/BP_/WIdget/Enemy/WBP_HealthBarEnemy.TextBlock_EnemyName` (cast `/Game/Like/BP_/WIdget/Enemy/WBP_HealthBarEnemy` (`WidgetComponent.GetWidget` (`self.WidgetComponent`)) :!pure true)) "불량배"))

(event `self.ReceiveHit`
  (params (MyComp :type "PrimitiveComponent Object Reference") (Other :type "Actor Object Reference") (OtherComp :type "PrimitiveComponent Object Reference") (bSelfMoved :type Boolean) (HitLocation :type "Vector Structure") (HitNormal :type "Vector Structure") (NormalImpulse :type "Vector Structure") (Hit :type "HitResult Structure (by ref)"))
  ;[1 1 1] 원거리 적 검에 맞을시 머티리얼 변경 테스트
  (`PrimitiveComponent.SetMaterialByName` (`self.Mesh`) "MI_c_am_com_haka_kyaha_kimono" "/Game/Asset/Character/NPC/Man/Ryonin1/Material/MI_TEST.MI_TEST")
  (`KismetSystemLibrary.Delay` 0.2)
  (`PrimitiveComponent.SetMaterialByName` (`self.Mesh`) "MI_c_am_com_haka_kyaha_kimono" "/Game/Asset/Character/NPC/Man/Ryonin1/Material/MI_c_am_com_haka_kyaha_kimono.MI_c_am_com_haka_kyaha_kimono"))

(fn `UserConstructionScript`
  (`parent.UserConstructionScript`))