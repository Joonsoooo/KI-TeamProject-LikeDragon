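; BP_Boss is the boss enemy Okita Soji, extending a parent enemy class.
; On BeginPlay it writes the boss name to the enemy health bar widget and switches off its two aura effects.
; The OnHealthBelow50 event activates both auras.
; ChangeWeaponNotify snaps the left-hand weapon to the boss hand socket on the mesh, keeping its world scale.
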(event `self.ReceiveBeginPlay`
  (`parent.ReceiveBeginPlay`)
  (`TextBlock.SetText` (`/Game/Like/BP_/WIdget/Enemy/WBP_HealthBarEnemy.TextBlock_EnemyName` (cast `/Game/Like/BP_/WIdget/Enemy/WBP_HealthBarEnemy` (`WidgetComponent.GetWidget` (`self.WidgetComponent`)) :!pure true)) "오키타 소지")
  (`ActorComponent.Deactivate` (`self.NS_Aura_1_Boss`))
  (`ActorComponent.Deactivate` (`self.NS_Aura_2_Boss`)))

(event `OnHealthBelow50`
  (`ActorComponent.Activate` (`self.NS_Aura_1_Boss`) false)
  (`ActorComponent.Activate` (`self.NS_Aura_2_Boss`) false))

(event `ChangeWeaponNotify`
  (`self.AttachWeaponToHand`))

(fn `AttachWeaponToHand`
  (`self.K2_AttachToComponent` (`self.LeftHandWeapon`) (`self.Mesh`) "EquipHand_L_Boss" "SnapToTarget" "SnapToTarget" "KeepWorld" true))

(fn `UserConstructionScript`
  (`parent.UserConstructionScript`))