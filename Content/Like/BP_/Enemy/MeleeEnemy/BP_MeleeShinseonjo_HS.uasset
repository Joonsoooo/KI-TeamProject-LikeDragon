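; BP_MeleeShinseonjo_HS is a melee enemy Blueprint for the Shinseonjo (신선조) enemy, built on a parent class that supplies its behavior.
; On BeginPlay it runs the parent logic, then casts its WidgetComponent's widget to WBP_HealthBarEnemy and sets the displayed enemy name to "신선조".
; The construction script only calls the parent, and the overlap and Tick events are disabled.
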(event `self.ReceiveBeginPlay`
  (`parent.ReceiveBeginPlay`)
  (`TextBlock.SetText` (`/Game/Like/BP_/WIdget/Enemy/WBP_HealthBarEnemy.TextBlock_EnemyName` (cast `/Game/Like/BP_/WIdget/Enemy/WBP_HealthBarEnemy` (`WidgetComponent.GetWidget` (`self.WidgetComponent`)) :!pure true)) "신선조"))

(fn `UserConstructionScript`
  (`parent.UserConstructionScript`))